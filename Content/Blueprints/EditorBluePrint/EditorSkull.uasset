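; EditorSkull is a skull actor, apparently for editor use, whose skeletal mesh can be toggled.
; On BeginPlay it clears the SkullRef on every Obj_DD actor in the level.
; The Hide_Show event flips the Hide flag and swaps the mesh, assigning IdoAvatarMesh when Hide becomes true and no specified mesh when it becomes false.
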(event `self.ReceiveBeginPlay`
  ;[1 1 1] Init
  (bind _outactors (`GameplayStatics.GetAllActorsOfClass` "/Game/Blueprints/EditorBluePrint/Obj_DD.Obj_DD_C"))
  (for _array_element _outactors
    (set `/Game/Blueprints/EditorBluePrint/Obj_DD.skullRef` null _array_element)))

(event `Hide_Show`
  (bind _skeletalmeshcomponent (`self.SkeletalMeshComponent`))
  ;[1 1 1] Hide/Show skull
  (if (`self.Hide`)
    (set `self.Hide` false)
    (`SkinnedMeshComponent.SetSkinnedAssetAndUpdate` _skeletalmeshcomponent null)
    (else
      (set `self.Hide` true)
      (`SkinnedMeshComponent.SetSkinnedAssetAndUpdate` _skeletalmeshcomponent "/Game/Blueprints/AvatarBluePrint/IdoAvatarMesh.IdoAvatarMesh"))))

(fn `UserConstructionScript`)