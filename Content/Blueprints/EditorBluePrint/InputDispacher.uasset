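; Input dispatcher for a timeline-based note editor, routing mouse and key actions to the timeline, its notes, Obj_DD spawners and the EditorSkull.
; Left click grabs hovered notes or spawns from hovered Obj_DD actors, setting a moving flag cleared on release; right-click release goes to hovered notes.
; While moving, Tick pins the cursor to viewport center and wheel and mouse-axis input drive movable notes; otherwise the wheel scrolls the timeline.
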(event `self.ReceiveBeginPlay`
  (bind _outactors (`GameplayStatics.GetAllActorsOfClass` "/Game/Blueprints/EditorBluePrint/Obj_DD.Obj_DD_C"))
  (set `self.Obj_DD_Array` _outactors)
  (bind _outactors_2 (`GameplayStatics.GetAllActorsOfClass` "/Game/Blueprints/EditorBluePrint/EditorSkull.EditorSkull_C"))
  (for _array_element _outactors_2
    (set `self.SkullRef` _array_element)
    (`self.EnableInput` (`GameplayStatics.GetPlayerController` 0))))

(event `self.ReceiveTick`
  (params (DeltaSeconds :type "Float (single-precision)"))
  (bind _returnvalue (`GameplayStatics.GetPlayerController` 0))
  (bind (_posx _posy) (`VictoryBPFunctionLibrary.Viewport__GetCenterOfViewport` _returnvalue))
  (if (`self.Is_SimpleObj_Moving`)
    (`VictoryBPFunctionLibrary.Viewport__SetMousePosition` _returnvalue _posx _posy)))

(event `InputAction|ToMenu`
  (:`Pressed`
    (`/Game/Blueprints/EditorBluePrint/Timeline.Back` (`self.Timeline_Reference`))))

(event `InputAction|WheelUp`
  (:`Pressed`
    (if (`self.Is_SimpleObj_Moving`)
      (for _array_element (`/Game/Blueprints/EditorBluePrint/Timeline.noteArray` (`self.Timeline_Reference`))
        (if (`/Game/Blueprints/EditorBluePrint/simpleObj.Movable` _array_element)
          (`/Game/Blueprints/EditorBluePrint/simpleObj.IN_WheelUp` _array_element)))
      (else
        (`/Game/Blueprints/EditorBluePrint/Timeline.Left` (`self.Timeline_Reference`) :!label _label)))))

(event `InputAction|Right`
  (:`Pressed`
    (`/Game/Blueprints/EditorBluePrint/Timeline.Right` (`self.Timeline_Reference`) :!label _label_2)))

(event `InputAction|WheelDown`
  (:`Pressed`
    (if (`self.Is_SimpleObj_Moving`)
      (for _array_element (`/Game/Blueprints/EditorBluePrint/Timeline.noteArray` (`self.Timeline_Reference`))
        (if (`/Game/Blueprints/EditorBluePrint/simpleObj.Movable` _array_element)
          (`/Game/Blueprints/EditorBluePrint/simpleObj.IN_WheelDown` _array_element)))
      (else
        (goto _label_2)))))

(event `InputAction|Left`
  (:`Pressed`
    (goto _label)))

(event `InputAction|Reset`
  (:`Pressed`
    (`/Game/Blueprints/EditorBluePrint/Timeline.Reset` (`self.Timeline_Reference`))))

(event `InputAxis|MouseX`
  (params (AxisValue :type "Float (single-precision)"))
  (if (`self.Is_SimpleObj_Moving`) :!label _label_3
    (for _array_element (`/Game/Blueprints/EditorBluePrint/Timeline.noteArray` (`self.Timeline_Reference`))
      (if (`/Game/Blueprints/EditorBluePrint/simpleObj.Movable` _array_element)
        (`/Game/Blueprints/EditorBluePrint/simpleObj.RefreshMouseAxis` _array_element AxisValue (stale `InputAxis|MouseY` AxisValue))))))

(event `InputAxis|MouseY`
  (params (AxisValue :type "Float (single-precision)"))
  (goto _label_3))

(event `InputAction|HideSkull`
  (:`Pressed`
    (`/Game/Blueprints/EditorBluePrint/EditorSkull.Hide_Show` (`self.skullRef`))))

(event `InputAction|LeftClic`
  (bind _is_simpleobj_moving (`self.Is_SimpleObj_Moving`))
  (:`Pressed`
    (if (not _is_simpleobj_moving)
      (for _array_element (`/Game/Blueprints/EditorBluePrint/Timeline.noteArray` (`self.Timeline_Reference`))
        (if (`/Game/Blueprints/EditorBluePrint/simpleObj.MouseOver` _array_element)
          (`/Game/Blueprints/EditorBluePrint/simpleObj.LeftClicPressed` _array_element)
          (set `self.Is_SimpleObj_Moving` true)))
      (bind _outactors (`GameplayStatics.GetAllActorsOfClass` "/Game/Blueprints/EditorBluePrint/Obj_DD.Obj_DD_C"))
      (for _array_element_2 _outactors
        (if (`/Game/Blueprints/EditorBluePrint/Obj_DD.MouseOver` _array_element_2)
          (`/Game/Blueprints/EditorBluePrint/Obj_DD.Spawn` _array_element_2)
          (set `self.Is_SimpleObj_Moving` true)))))
  (:`Released`
    (if _is_simpleobj_moving
      (for _array_element_3 (`/Game/Blueprints/EditorBluePrint/Timeline.noteArray` (`self.Timeline_Reference`))
        (if (`/Game/Blueprints/EditorBluePrint/simpleObj.Movable` _array_element_3)
          (`/Game/Blueprints/EditorBluePrint/simpleObj.LeftClicRelease` _array_element_3)
          (set `self.Is_SimpleObj_Moving` false))))))

(event `InputAction|RightClic`
  (:`Released`
    (for _array_element (`/Game/Blueprints/EditorBluePrint/Timeline.noteArray` (`self.Timeline_Reference`))
      (if (`/Game/Blueprints/EditorBluePrint/simpleObj.MouseOver` _array_element)
        (`/Game/Blueprints/EditorBluePrint/simpleObj.RightClicPressed` _array_element)))))

(fn `UserConstructionScript`)