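; Editor note object on a beat timeline, shown as a sphere that can be dragged or deleted with the mouse.
; RefreshTimer reads the timeline's Beat to show it from spawn lead-in through duration, blue before its active time and red after.
; While held, Tick applies mouse axes to X/Z and wheel steps set Y; release clamps it to the timeline's bounds.
; Right-click removes it from NoteArray, rechecks the highest beat and destroys it.
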(event Custom|RefreshTimer
  (bind _staticmeshcomponent (Variables|Debug|GetStaticMeshComponent))
  ;[1 1 1] TimeManager
  (bind _output_get (Variables|Default|SetGlobalTimer (Variables|/Game/Blueprints/EditorBluePrint/Timeline.Timeline_C|GetBeat (Variables|Default|GettimelineRef))))
  (bind _output_get_2 (Variables|Default|SetVisible (|((a>=b)&&(a<c)) _output_get (- (Variables|Default|GetActiveTime) (Variables|Default|GetSpawnTime)) (+ (Variables|Default|GetActiveTime) (Variables|Default|GetDuration)))))
  (if _output_get_2
    (Rendering|SetVisibility _staticmeshcomponent true true)
    (Components|StaticMesh|SetStaticMesh _staticmeshcomponent "/Game/Asset/EditorAsset/sphere.sphere")
    ;[1 1 1] ColorSwitch
    (if (|(a&&b) (Variables|Default|GetVisible) (< (Variables|Default|GetGlobalTimer) (Variables|Default|GetActiveTime)))
      (Rendering|Material|SetMaterial (Variables|Debug|GetStaticMeshComponent) 0 "/Game/material/Blue.Blue")
      (elif (|(a&&b) (Variables|Default|GetVisible) (>= (Variables|Default|GetGlobalTimer) (Variables|Default|GetActiveTime)))
        (Rendering|Material|SetMaterial (Variables|Debug|GetStaticMeshComponent) 0 "/Game/material/Red.Red")))
    (else
      (Rendering|SetVisibility _staticmeshcomponent false true)
      (Components|StaticMesh|SetStaticMesh _staticmeshcomponent 0))))

(event Custom|IN_WheelDown
  ;[1 1 1] Drag&Drop
  (if (Variables|Default|GetMovable)
    (Variables|Default|SetvY (+ (Variables|Default|GetvY) -5e+01))))

(event Custom|IN_WheelUp
  ;[1 1 1] Drag&Drop
  (if (Variables|Default|GetMovable)
    (Variables|Default|SetvY (+ (Variables|Default|GetvY) 5e+01))))

(event Custom|LeftClicRelease
  (bind _returnvalue (Transformation|GetActorLocation))
  (bind _returnvalue_2 (Transformation|GetActorLocation))
  (bind _timelineref (Variables|Default|GettimelineRef))
  (bind _timelineref_2 (Variables|Default|GettimelineRef))
  (bind (_x _y _z) (Math|Vector|BreakVector _returnvalue))
  (bind (_x_2 _y_2 _z_2) (Math|Vector|BreakVector _returnvalue_2))
  (bind _origin (Variables|/Game/Blueprints/EditorBluePrint/Timeline.Timeline_C|Getorigin _timelineref))
  (bind _maxarea (Variables|/Game/Blueprints/EditorBluePrint/Timeline.Timeline_C|GetMaxArea _timelineref_2))
  (bind (_x_3 _y_3 _z_3) (Math|Vector|BreakVector _maxarea))
  (bind (_x_4 _y_4 _z_4) (Math|Vector|BreakVector _origin))
  ;[1 1 1] Drag&Drop
  (Variables|Default|SetMovable false)
  (Variables|/Script/Engine.PlayerController|SetbShowMouseCursor (Game|GetPlayerController 0) true)
  ;[1 1 1] Snap
  (if (> _x_2 _x_4)
    (Transformation|SetActorLocation (Math|Vector|MakeVector _x_4 _y_2 _z_2) false))
  (if (< _z_2 _z_4)
    (Transformation|SetActorLocation (Math|Vector|MakeVector _x_2 _y_2 _z_4) false))
  (if (> _y_2 _y_4)
    (Transformation|SetActorLocation (Math|Vector|MakeVector _x_2 _y_4 _z_2) false)
    (Variables|Default|SetvY _y_4))
  (if (< _x _x_3)
    (Transformation|SetActorLocation (Math|Vector|MakeVector _x_3 _y _z) false))
  (if (> _z _z_3)
    (Transformation|SetActorLocation (Math|Vector|MakeVector _x _y _z_3) false))
  (if (< _y _y_3)
    (Transformation|SetActorLocation (Math|Vector|MakeVector _x _y_3 _z) false)
    (Variables|Default|SetvY _y_3)))

(event Custom|RightClicPressed
  (bind _timelineref (Variables|Default|GettimelineRef))
  ;[1 1 1] Delete
  (if (Variables|Default|GetVisible)
    (Variables|/Script/Engine.PlayerController|SetbShowMouseCursor (Game|GetPlayerController 0) true)
    (Utilities|Array|RemoveItem (Variables|/Game/Blueprints/EditorBluePrint/Timeline.Timeline_C|GetnoteArray _timelineref) self)
    (Default|CheckHighestBeat _timelineref)
    (Actor|DestroyActor)))

(event Custom|RefreshMouseAxis
  (params (X :type Float%20%28single-precision%29) (Y :type Float%20%28single-precision%29))
  ;[1 1 1] Drag&Drop
  (Variables|Default|SetMouseXaxis X)
  (Variables|Default|SetMouseYaxis Y))

(event Custom|LeftClicPressed
  ;[1 1 1] Drag&Drop
  (if (Variables|Default|GetVisible)
    (Variables|Default|SetMovable true)
    (Variables|/Script/Engine.PlayerController|SetbShowMouseCursor (Game|GetPlayerController 0) false)))

(event EventTick
  (params (DeltaSeconds :type Float%20%28single-precision%29))
  (bind _returnvalue (Transformation|GetActorLocation))
  (bind (_x _y _z) (Math|Vector|BreakVector _returnvalue))
  ;[1 1 1] Drag&Drop
  (if (Variables|Default|GetMovable)
    (Transformation|SetActorLocation (|((a*b)+c) (Math|Vector|MakeVector (Variables|Default|GetMouseXaxis) 0.0 (Variables|Default|GetMouseYaxis)) 1e+01 (Math|Vector|MakeVector _x (Variables|Default|GetvY) _z)) false)))

(event EventBeginPlay
  (bind _staticmeshcomponent (Variables|Debug|GetStaticMeshComponent))
  ;[1 1 1] Init
  ;[1 1 1] TimeManager
  (if (stale Custom|RefreshTimer _output_get_2)
    (Rendering|SetVisibility _staticmeshcomponent true true)
    (Components|StaticMesh|SetStaticMesh _staticmeshcomponent "/Game/Asset/EditorAsset/sphere.sphere")
    ;[1 1 1] ColorSwitch
    (if (|(a&&b) (Variables|Default|GetVisible) (< (Variables|Default|GetGlobalTimer) (Variables|Default|GetActiveTime)))
      (Rendering|Material|SetMaterial (Variables|Debug|GetStaticMeshComponent) 0 "/Game/material/Blue.Blue")
      (elif (|(a&&b) (Variables|Default|GetVisible) (>= (Variables|Default|GetGlobalTimer) (Variables|Default|GetActiveTime)))
        (Rendering|Material|SetMaterial (Variables|Debug|GetStaticMeshComponent) 0 "/Game/material/Red.Red")))
    (else
      (Rendering|SetVisibility _staticmeshcomponent false true)
      (Components|StaticMesh|SetStaticMesh _staticmeshcomponent 0))))

(event MouseInput|EventActorBeginCursorOver
  ;[1 1 1] Delete
  (Variables|Default|SetMouseOver true))

(event MouseInput|EventActorEndCursorOver
  ;[1 1 1] Delete
  (Variables|Default|SetMouseOver false))

(fn ConstructionScript)