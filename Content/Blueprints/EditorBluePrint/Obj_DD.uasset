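; Obj_DD is a level-editor actor that places SimpleObj notes on a beat-based timeline and tracks whether the cursor is over it.
; Its Spawn event creates an enlarged SimpleObj at its location, passing the timeline, current beat, duration and itself as parent.
; It then hides the mouse cursor, adds the note to the timeline's NoteArray and raises HighestBeat if the current beat exceeds it.
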(event `self.ReceiveActorBeginCursorOver`
  (set `self.MouseOver` true))

(event `self.ReceiveActorEndCursorOver`
  (set `self.MouseOver` false))

(event `Spawn`
  (bind _timelinerefblbl (`self.timelineRefblbl`))
  (bind _timelinerefblbl_2 (`self.timelineRefblbl`))
  (bind _beat (`/Game/Blueprints/EditorBluePrint/Timeline.Beat` _timelinerefblbl_2))
  ;[1 1 1] SimpleObjSpawn
  (bind _returnvalue (`|SpawnActorFromClass` "/Game/Blueprints/EditorBluePrint/simpleObj.simpleObj_C" (`KismetMathLibrary.MakeTransform` (`self.K2_GetActorLocation`) (struct) (1.5 1.5 1.5))))
  (set `/Game/Blueprints/EditorBluePrint/simpleObj.timelineRef` _timelinerefblbl_2 _returnvalue)
  (set `/Game/Blueprints/EditorBluePrint/simpleObj.GlobalTimer` _beat _returnvalue)
  (set `/Game/Blueprints/EditorBluePrint/simpleObj.ActiveTime` _beat _returnvalue)
  (set `/Game/Blueprints/EditorBluePrint/simpleObj.Dad` self _returnvalue)
  (set `/Game/Blueprints/EditorBluePrint/simpleObj.Duration` (`self.Duration`) _returnvalue)
  (set `PlayerController.bShowMouseCursor` false (`GameplayStatics.GetPlayerController` 0))
  (`KismetArrayLibrary.Array_Add` (`/Game/Blueprints/EditorBluePrint/Timeline.noteArray` (`self.timelineRefblbl`)) _returnvalue)
  (if (> _beat (`/Game/Blueprints/EditorBluePrint/Timeline.HighestBeat` _timelinerefblbl))
    (set `/Game/Blueprints/EditorBluePrint/Timeline.HighestBeat` _beat _timelinerefblbl)))

(fn `UserConstructionScript`)