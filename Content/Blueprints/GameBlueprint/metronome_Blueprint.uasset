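; Metronome actor that pulses its scale and plays kick sounds in time with the BPM read from the first Floor_Blueprint.
; BeginPlay starts a timeline offset by game time, and Tick applies its track as actor scale with play rate tied to BPM.
; Math expressions compare accumulated time to a beat counter to trigger each kick, using a different sample every fourth beat.
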(event EventBeginPlay
  ;[1 1 1] create a timeline according to the bpm
  (bind _outactors (Actor|GetAllActorsOfClass "/Game/Blueprints/GameBlueprint/Floor_Blueprint.Floor_Blueprint_C"))
  (Variables|Default|SetBpm (Math|Conversions|ToFloat(Integer) (Variables|/Game/Blueprints/GameBlueprint/Floor_Blueprint.Floor_Blueprint_C|GetBPM (Utilities|Array|Get(acopy) _outactors))))
  (Utilities|FlowControl|Sequence
    (:then_0
      (bind _newtrack_0 (Timeline|Timeline_0 SetNewTime)))
    (:then_1
      (Timeline|Timeline_0 Play))))

(event EventTick
  (params (DeltaSeconds :type Float%20%28single-precision%29))
  (bind _returnvalue (Transformation|GetActorLocation))
  ;[1 1 1] play the tick sound in rhythm
  (Variables|Default|SetTime (+ (Variables|Default|GetTime) DeltaSeconds))
  (Transformation|SetActorScale3D (Math|Conversions|ToVector(Float) (stale EventBeginPlay _newtrack_0)))
  (Components|Timeline|SetPlayRate (Variables|Default|GetTimeline_0) (/ (Variables|Default|GetBpm) 6e+01))
  (if (|(({AB37842B-4D37-7768-0382-77976E98C354}/(60/{4D70D3EE-4F88-EE52-36D2-238B0C38E6EB}))>{EBB369C9-4A7F-442E-D20B-7F9DE75BFC53}))
    (if (|(({EBB369C9-4A7F-442E-D20B-7F9DE75BFC53}%4)==0))
      (Audio|PlaySoundatLocation "/Game/Sounds/phony-ppl_kick-2_drums_one_shot_121_wav.phony-ppl_kick-2_drums_one_shot_121_wav" _returnvalue)
      (else
        (Audio|PlaySoundatLocation "/Game/Sounds/phony-ppl_kick-1_drums_one_shot_121_wav.phony-ppl_kick-1_drums_one_shot_121_wav" _returnvalue)))
    (Variables|Default|SetBeat (+ (Math|Float|Truncate (|({AB37842B-4D37-7768-0382-77976E98C354}/(60/{4D70D3EE-4F88-EE52-36D2-238B0C38E6EB})))) 1))))

(fn ConstructionScript)