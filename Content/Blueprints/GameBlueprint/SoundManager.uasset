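; Short-lived sound actor that plays a note once, with a fail variant, then fades out and destroys itself.
; BeginPlay assigns RandomNote to the audio component, and PlayNote or PlayFailSound starts it if not already playing.
; On failure, Tick lowers the PitchFade parameter until a threshold triggers the ending, which End also triggers directly.
; Ending drives Vol from a timeline curve whose time Tick sets manually, destroying the actor when the countdown expires.
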(event `PlayNote`
  ;[1 1 1] Play
  (if (not (`self.IsPlaying`)) :!label _label
    (`AudioComponent.Play` (`self.Audio`) 0.0)
    (set `self.IsPlaying` true)))

(event `self.ReceiveBeginPlay`
  ;[1 1 1] Init
  (bind _output_get (set `self.Sound` "/Game/Sounds/RandomNote.RandomNote"))
  (set `AudioComponent.Sound` _output_get (`self.Audio`))
  (set `self.Param` 1.0)
  (set `self.Param2` 1.0))

(event `PlayFailSound`
  ;[1 1 1] Play
  (set `self.FailBool` true)
  (goto _label))

(event `End`
  ;[1 1 1] Play
  (set `self.EndBool` true))

(event `self.ReceiveTick`
  (params (DeltaSeconds :type "Float (single-precision)"))
  (bind _returnvalue (* 2 DeltaSeconds))
  (bind _param2 (`self.Param2`))
  (bind _param (`self.Param`))
  (bind _returnvalue_2 (- _param _returnvalue))
  ;[1 1 1] End
  (if (`self.FailBool`)
    (bind _output_get (set `self.Param2` (- _param2 _returnvalue)))
    (`AudioComponent.SetFloatParameter` (`self.Audio`) "PitchFade" _output_get)
    (if (< _param2 0.7)
      (set `self.EndBool` true)))
  (if (`self.EndBool`)
    (bind (_direction _curve) (`Timeline|Timeline_0` :`NewTime` _returnvalue_2 :!via `SetNewTime`)
      (:`Update`
        (set `self.Param` _returnvalue_2)
        (`AudioComponent.SetFloatParameter` (`self.Audio`) "Vol" _curve)
        (if (< _param 0.0)
          (`self.K2_DestroyActor`))))))

(fn `UserConstructionScript`)