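; Spawning_Light is an actor that carries a particle effect around a small wobbling orbit, and its graph notes it may no longer be used.
; BeginPlay attaches the emitter to the static mesh, then stores the start position and a random time offset.
; Tick uses game time in sine and cosine to circle that position in the XZ plane, re-randomizing the radius each frame and forcing world Y to zero.
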(event EventBeginPlay
  (bind _returnvalue (Transformation|GetActorLocation))
  ;[1 1 1] not used anymore ?
  (Effects|SpawnEmitterAttached "/Game/Particles/particles.particles" (Variables|Default|GetStaticMeshComponent0) "None" _returnvalue "0, 0, 0" "KeepRelativeOffset" false)
  (Variables|Default|Setinitial_pos _returnvalue)
  (Variables|Default|Setrandom (Math|Random|RandomFloat)))

(event EventTick
  (params (DeltaSeconds :type Float%20%28single-precision%29))
  (bind _returnvalue (Utilities|Time|GetGameTimeinSeconds))
  (bind _returnvalue_2 (Math|Random|RandomFloatinRange 4e+01 5e+01))
  (bind _random (Variables|Default|Getrandom))
  (bind _initial_pos (Variables|Default|Getinitial_pos))
  (bind (_x _y _z) (Math|Vector|BreakVector _initial_pos))
  (bind _returnvalue_3 (+ _returnvalue _random))
  (bind _returnvalue_4 (* _returnvalue_3 2.0))
  ;[1 1 1] not used anymore ?
  (Transformation|SetActorLocation (Math|Vector|MakeVector (+ (* (|(cos(x)) _returnvalue_4) _returnvalue_2) _x) 0.0 (+ (* (|(sin(x)) _returnvalue_4) _returnvalue_2) _z)) false))

(fn ConstructionScript)