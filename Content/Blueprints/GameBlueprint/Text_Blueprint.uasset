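; Floating score text actor that pops up on targets and removes itself once its TimeLeft countdown runs out.
; On the first Tick with empty text it sets a fixed rotation, writes ScoreText into the TextRender and colors it red when Points is zero.
; A Timeline started on BeginPlay supplies a Translation value that Tick adds to the current Z each frame, so the vertical movement accumulates and depends on frame rate.
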(event `self.ReceiveTick`
  (params (DeltaSeconds :type "Float (single-precision)"))
  (bind _textrender (`self.TextRender`))
  (`|ExecutionSequence`
    (:`then_0`
      ;[1 1 1] Manage text appearing on the targets
      (if (`KismetTextLibrary.TextIsEmpty` (`TextRenderComponent.Text` (`self.TextRender`)))
        (`self.SetActorRotation` (struct :`Yaw` 90.0))
        (`TextRenderComponent.K2_SetText` _textrender (`KismetTextLibrary.Conv_StringToText` (`self.score_text`)))
        (if (== (`self.points`) 0)
          (`TextRenderComponent.SetTextRenderColor` _textrender (make `Color` 0 0 255)))))
    (:`then_1`
      ;[1 1 1] Destroy when finish
      (bind _output_get (set `self.time_left` (- (`self.time_left`) DeltaSeconds)))
      (if (< _output_get 0.0)
        (`self.K2_DestroyActor`)))
    (:`then_2`
      ;[1 1 1] Set location depending on time
      (`self.K2_SetActorLocation` (`KismetMathLibrary.MakeVector` (.x (`self.K2_GetActorLocation`)) (.y (`self.K2_GetActorLocation`)) (+ (.z (`self.K2_GetActorLocation`)) (stale `self.ReceiveBeginPlay` _translation)))))))

(event `self.ReceiveBeginPlay`
  ;[1 1 1] Set location depending on time
  (bind (_direction _translation) (`Timeline|Timeline_0`)))

(fn `UserConstructionScript`)