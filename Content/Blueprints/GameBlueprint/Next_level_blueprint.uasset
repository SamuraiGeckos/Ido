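; Level-exit actor that advances the game to the next text-file level when any actor begins overlapping it.
; It reads the current name from selectedLevel.txt, finds it in the levels folder listing and writes back the following file's name without extension, using Victory plugin file IO.
; It then reopens the Game map, with that file carrying the selection.
; The index has no bounds check, and selectedLevel.txt shares the listed folder.
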(event `self.ReceiveActorBeginOverlap`
  (params (OtherActor :type "Actor Object Reference"))
  (bind _files (`VictoryBPFunctionLibrary.JoyFileIO_GetFiles` (`VictoryBPFunctionLibrary.AppendMultiple` (`VictoryBPFunctionLibrary.VictoryPaths__GameRootDirectory`) "/levels/")))
  ;[1 1 1] find wich is the next level and open it
  (`VictoryBPFunctionLibrary.FileIO__SaveStringTextToFile` (`KismetStringLibrary.Concat_StrStr` (`VictoryBPFunctionLibrary.VictoryPaths__GameRootDirectory`) "/levels") "selectedLevel.txt" (`KismetStringLibrary.Replace` (`KismetArrayLibrary.Array_Get` _files (+ (`KismetArrayLibrary.Array_Find` _files (`KismetStringLibrary.Concat_StrStr` (`KismetArrayLibrary.Array_Get` (`VictoryBPFunctionLibrary.LoadStringArrayFromFile` (`VictoryBPFunctionLibrary.AppendMultiple` (`VictoryBPFunctionLibrary.VictoryPaths__GameRootDirectory`) "/levels/selectedLevel.txt"))) ".txt")) 1)) ".txt") true)
  (`GameplayStatics.OpenLevel` "Game"))

(fn `UserConstructionScript`)