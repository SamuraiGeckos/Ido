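; Timed target sphere for a rhythm-style game, scoring how close to zero on its countdown the player touches it.
; BeginPlay spawns a timeline-scaled child sphere, a spotlight and a SoundManager; Tick counts down, then plays the note or signals failure past the margin.
; Overlap grades timing, adds to Floor_Blueprint's score and drives color, text, particle and light feedback.
; Overlap at spawn warns "GO OUT"; untouched targets show "MISSED" on destruction.
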(event Custom|OnActorDestroy
  ;[1 1 1] If the player miss the target
  (Default|End (Variables|Default|GetsoundManagerRef))
  (Actor|DestroyActor (Variables|Default|GetSpotlightRef))
  (if (<= (Variables|Default|Getscore_on_this_frame) 0)
    (if (not (Variables|Default|GetOverlapEvent))
      (Variables|Default|Setscore_quality "MISSED")
      (bind _returnvalue (Game|SpawnActorfromClass "/Game/Blueprints/GameBlueprint/Text_Blueprint.Text_Blueprint_C" (Math|Conversions|ToTransform(Vector) (Transformation|GetActorLocation)) false 0 0))
      (Variables|/Game/Blueprints/GameBlueprint/Text_Blueprint.Text_Blueprint_C|Setscore_text _returnvalue (Variables|Default|Getscore_quality)))))

(event EventBeginPlay
  (bind _returnvalue (Transformation|GetActorLocation))
  (bind _returnvalue_2 (Math|Conversions|ToTransform(Vector) _returnvalue))
  (bind (_x _y) (Math|Vector|BreakVector _returnvalue))
  ;[1 1 1] initialization
  (bind _returnvalue_3 (Game|SpawnActorfromClass "/Game/Blueprints/GameBlueprint/Sphere_child.Sphere_child_C" _returnvalue_2 false 0 0))
  (Variables|Default|Setsphere_child_ref _returnvalue_3)
  (bind _returnvalue_4 (Game|SpawnActorfromClass "/Game/Blueprints/GameBlueprint/SoundManager.SoundManager_C" _returnvalue_2 false 0 0))
  (Variables|Default|SetsoundManagerRef _returnvalue_4)
  (bind _returnvalue_5 (Game|SpawnActorfromClass "/Game/Blueprints/GameBlueprint/SpotLight_target_Blueprint.SpotLight_target_Blueprint_C" (Math|Transform|MakeTransform (Math|Vector|MakeVector _x _y 1.5e+02) "-90.000000, 0, 0" "1.000000,1.000000,1.000000") false 0 0))
  (Variables|Default|SetSpotlightRef _returnvalue_5)
  (Transformation|SetActorScale3D "1.500000,1.500000,1.500000")
  (bind _newtrack_1 (Timeline|Timeline_1 Play)))

(event Collision|EventActorEndOverlap
  (params (OtherActor :type Actor%20Object%20Reference))
  ;[1 1 1] If the player is already in the target when it spawns
  (if (== (Variables|Default|GetOverlapYellow) 1)
    (Rendering|Material|SetMaterial (Variables|Default|GetStaticMeshComponent0) 0 "/Game/material/TransparentBlue.TransparentBlue")
    (Rendering|Material|SetMaterial (Variables|/Game/Blueprints/GameBlueprint/Sphere_child.Sphere_child_C|GetStaticMeshComponent0 (Variables|Default|Getsphere_child_ref)) 0 "/Game/material/TransparentBlue.TransparentBlue")
    (Actor|DestroyActor (stale Collision|EventActorBeginOverlap _returnvalue_8))))

(event Collision|EventActorBeginOverlap
  (params (OtherActor :type Actor%20Object%20Reference))
  (bind _self self)
  (bind _marge (Variables|Default|GetMarge))
  (bind _active_time_left (Variables|Default|Getactive_time_left))
  (bind _active_time_left_2 (Variables|Default|Getactive_time_left))
  (bind _returnvalue (* -1 _marge))
  (bind _returnvalue_2 (Transformation|GetActorLocation _self))
  (bind _returnvalue_3 (Math|Float|Clamp(Float) _active_time_left _returnvalue _marge))
  (bind _returnvalue_4 (Math|Float|Absolute(Float) _returnvalue_3))
  (bind _returnvalue_5 (- _marge _returnvalue_4))
  (bind _returnvalue_6 (* _returnvalue_5 4e+02))
  (bind _returnvalue_7 (Math|Float|Truncate _returnvalue_6))
  ;[1 1 1] general sphere management : score, color, display, etc
  (if (== (Variables|Default|Getactive_time_left) 1.0)
    ;[1 1 1] If the player is already in the target when it spawns
    (Variables|Default|SetOverlapYellow 1)
    (Rendering|Material|SetMaterial (Variables|Default|GetStaticMeshComponent0) 0 "/Game/material/TransparentYellow.TransparentYellow")
    (Rendering|Material|SetMaterial (Variables|/Game/Blueprints/GameBlueprint/Sphere_child.Sphere_child_C|GetStaticMeshComponent0 (Variables|Default|Getsphere_child_ref)) 0 "/Game/material/TransparentYellow.TransparentYellow")
    (Variables|Default|Setscore_quality "GO OUT")
    (bind _returnvalue_8 (Game|SpawnActorfromClass "/Game/Blueprints/GameBlueprint/Text_Blueprint2.Text_Blueprint2_C" (Math|Conversions|ToTransform(Vector) (Transformation|GetActorLocation self)) false 0 0))
    (Variables|/Game/Blueprints/GameBlueprint/Text_Blueprint2.Text_Blueprint2_C|Setscore_text2 _returnvalue_8 (Variables|Default|Getscore_quality))
    (else
      (Variables|Default|SetOverlapYellow 0)
      (Variables|Default|Setactive false)
      (Utilities|FlowControl|DoOnce false
        (:Completed
          (Actor|DestroyActor (Variables|Default|Getsphere_child_ref))
          (bind _outactors (Actor|GetAllActorsOfClass "/Game/Blueprints/GameBlueprint/Floor_Blueprint.Floor_Blueprint_C"))
          (Variables|/Game/Blueprints/GameBlueprint/Floor_Blueprint.Floor_Blueprint_C|Setscore (Utilities|Array|Get(acopy) _outactors) (+ (Variables|/Game/Blueprints/GameBlueprint/Floor_Blueprint.Floor_Blueprint_C|Getscore (Utilities|Array|Get(acopy) _outactors)) _returnvalue_7))
          (Variables|Default|Setscore_on_this_frame _returnvalue_7)
          (if (> _returnvalue_7 90)
            (Variables|Default|Setscore_quality "PERFECT")
            (Rendering|Material|SetMaterial (Variables|Default|GetStaticMeshComponent0) 0 "/Game/material/TransparentGreen.TransparentGreen" :!label _label)
            (Rendering|Components|Light|SetLightColor (Variables|/Script/Engine.SpotLight|GetSpotLightComponent (Variables|Default|GetSpotlightRef)) "(R=0.000000,G=1.000000,B=0.000000,A=1.000000)")
            (bind _returnvalue_9 (Game|SpawnActorfromClass "/Game/Blueprints/GameBlueprint/Text_Blueprint.Text_Blueprint_C" (Math|Conversions|ToTransform(Vector) _returnvalue_2) false 0 0))
            (Variables|/Game/Blueprints/GameBlueprint/Text_Blueprint.Text_Blueprint_C|Setpoints _returnvalue_9 (Variables|Default|Getscore_on_this_frame))
            (Variables|/Game/Blueprints/GameBlueprint/Text_Blueprint.Text_Blueprint_C|Setscore_text _returnvalue_9 (Variables|Default|Getscore_quality))
            (Effects|SpawnEmitteratLocation "/Game/Particles/particles3.particles3" _returnvalue_2)
            (Effects|SpawnEmitteratLocation "/Game/Particles/particles4.particles4" (Math|Vector|MakeVector (Math|Random|RandomFloatinRange -1.1e+03 1.25e+03) (Math|Random|RandomFloatinRange -6.4e+02 -5.33e+03) (Math|Random|RandomFloatinRange 0.0 1.1e+03)))
            (bind _outactors_2 (Actor|GetAllActorsOfClass "/Game/Blueprints/GameBlueprint/Light_Blueprint.Light_Blueprint_C"))
            (Rendering|Components|Light|SetIntensity (Variables|/Script/Engine.Light|GetLightComponent (Utilities|Array|Get(acopy) _outactors_2)) (+ (Variables|/Script/Engine.LightComponentBase|GetIntensity (Variables|/Script/Engine.Light|GetLightComponent (Utilities|Array|Get(acopy) _outactors_2))) 3e+03))
            (elif (> _returnvalue_7 70)
              (Variables|Default|Setscore_quality "GREAT")
              (goto _label)
              (elif (> _returnvalue_7 50)
                (Variables|Default|Setscore_quality "GOOD")
                (goto _label)
                (elif (> _returnvalue_7 0)
                  (Variables|Default|Setscore_quality "NOT BAD")
                  (goto _label)
                  (else
                    ;[1 1 1] if the player touch the target too late / too soon
                    (Rendering|Material|SetMaterial (Variables|Default|GetStaticMeshComponent0) 0 "/Game/material/TransparentRed.TransparentRed")
                    (Default|PlayFailSound (Variables|Default|GetsoundManagerRef))
                    (Rendering|Components|Light|SetLightColor (Variables|/Script/Engine.SpotLight|GetSpotLightComponent (Variables|Default|GetSpotlightRef)) "(R=1.000000,G=0.000000,B=0.000000,A=1.000000)")
                    (if (< _active_time_left_2 0.25)
                      (Variables|Default|Setscore_quality "TOO LATE")
                      (bind _returnvalue_10 (Game|SpawnActorfromClass "/Game/Blueprints/GameBlueprint/Text_Blueprint.Text_Blueprint_C" (Math|Conversions|ToTransform(Vector) (Transformation|GetActorLocation self)) false 0 0 :!label _label_2))
                      (Variables|/Game/Blueprints/GameBlueprint/Text_Blueprint.Text_Blueprint_C|Setscore_text _returnvalue_10 (Variables|Default|Getscore_quality))
                      (Variables|Default|SetOverlapEvent true)
                      (elif (> _active_time_left_2 0.25)
                        (Variables|Default|Setscore_quality "TOO SOON")
                        (goto _label_2)))))))))))))

(event EventTick
  (params (DeltaSeconds :type Float%20%28single-precision%29))
  ;[1 1 1] time management and events
  (bind _output_get (Variables|Default|Setactive_time_left (- (Variables|Default|Getactive_time_left) DeltaSeconds)))
  (if (< _output_get 0.0)
    (if (|(a&&b) (< _output_get (* -1 (Variables|Default|GetMarge))) (Variables|Default|Getactive))
      (Default|PlayFailSound (Variables|Default|GetsoundManagerRef))
      (Rendering|Material|SetMaterial (Variables|Default|GetStaticMeshComponent0) 0 "/Game/material/TransparentRed.TransparentRed")
      (Rendering|Components|Light|SetLightColor (Variables|/Script/Engine.SpotLight|GetSpotLightComponent (Variables|Default|GetSpotlightRef)) "(R=1.000000,G=0.000000,B=0.000000,A=1.000000)"))
    (Variables|Default|Settime_left (- (Variables|Default|Gettime_left) DeltaSeconds))
    (Default|PlayNote (Variables|Default|GetsoundManagerRef))
    (Actor|DestroyActor (Variables|Default|Getsphere_child_ref))
    (else
      (Transformation|SetActorScale3D (Variables|Default|Getsphere_child_ref) (Math|Conversions|ToVector(Float) (stale EventBeginPlay _newtrack_1))))))

(fn ConstructionScript)