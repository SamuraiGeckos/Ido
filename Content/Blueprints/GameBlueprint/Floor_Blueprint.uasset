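; Floor actor that runs a rhythm level, spawning timed target spheres and showing the end menu.
; BeginPlay loads the selected level's text file into BPM, length and a flat five-float-per-target array.
; Tick converts game time to quarter-beat steps, spawns spheres four steps early, removes their entries and destroys expired spheres.
; Once the level length passes, it reveals the menu mesh and enables its children's overlaps.
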(event EventBeginPlay
  ;[1 1 1] Read file into float array
  ;;[1 1 1] Read file and put all the data is the "data" array
  (bind _output_get (Variables|Default|Setdata (.StringArray (Class|VictoryBPFunctionLibrary|LoadStringArrayfromFile (Utilities|String|Append (Class|VictoryBPFunctionLibrary|VictoryPathsGameRootDirectory) "/levels/" (Utilities|Array|Get(acopy) (.StringArray (Class|VictoryBPFunctionLibrary|LoadStringArrayfromFile (Class|VictoryBPFunctionLibrary|AppendMultiple (Class|VictoryBPFunctionLibrary|VictoryPathsGameRootDirectory) "/levels/selectedLevel.txt") false))) ".txt") false))))
  ;;[1 1 1] Save BPM and lenght of the level, then remove them from data
  (Variables|Default|SetBPM (Math|Conversions|ToInteger(Byte) (Utilities|Array|Get(acopy) (Utilities|String|ParseIntoArray (Utilities|Array|Get(acopy) _output_get) " "))))
  (Variables|Default|SetLenght (|(a-(12*(60/{A13BAC89-431D-964C-F8A2-F6920D9EFC22}))) (Math|Conversions|ToInteger(Byte) (Utilities|Array|Get(acopy) (Utilities|String|ParseIntoArray (Utilities|Array|Get(acopy) _output_get) " ") 1))))
  (Utilities|Array|RemoveIndex _output_get)
  (Utilities|Array|RemoveIndex (Variables|Default|Getdata) (Utilities|Array|LastIndex (Variables|Default|Getdata)))
  ;;[1 1 1] for each line of all the datas
  (for _array_element (Variables|Default|Getdata)
    (Utilities|Array|Clear (Variables|Default|Gettarget_info))
    (Utilities|Array|Clear (Variables|Default|Gettarget_position))
    ;;[1 1 1] save x,y,z positions
    (for _index (range 0 2)
      (Utilities|Array|Add (Variables|Default|Gettarget_position) (Math|Conversions|ToFloat(Integer) (Utilities|String|GetSubstring (Utilities|Array|Get(acopy) (Utilities|String|ParseIntoArray _array_element " ") _index) 2 8))))
    ;;[1 1 1] save duration and spawn time
    (for _index_2 (range 3 4)
      (Utilities|Array|Add (Variables|Default|Gettarget_info) (Math|Conversions|ToFloat(Integer) (Utilities|Array|Get(acopy) (Utilities|String|ParseIntoArray _array_element " ") _index_2))))
    (Utilities|Array|AppendArray (Variables|Default|Gettarget_info) (Variables|Default|Gettarget_position))
    ;;[1 1 1] "All targets" contains every targets info in that order: duration, spawn time, X,Y,Z
    (Utilities|Array|AppendArray (Variables|Default|Getall_targets) (Variables|Default|Gettarget_info))))

(event EventTick
  (params (DeltaSeconds :type Float%20%28single-precision%29))
  (bind _staticmeshcomponent (Variables|Debug|GetStaticMeshComponent))
  (bind _all_targets (Variables|Default|Getall_targets))
  (Utilities|FlowControl|Sequence
    (:then_0
      ;[1 1 1] Use the data from the "all targets" array and exploit them
      (for _index (range 0 (- (/ (Utilities|Array|Length (Variables|Default|Getall_targets)) 5) 1))
        (if (> (- (/ (Utilities|Time|GetGameTimeinSeconds) (/ 15.0 (Math|Conversions|ToFloat(Integer) (Variables|Default|GetBPM)))) -4.0) (Utilities|Array|Get(acopy) _all_targets (+ (* _index 5) 1)))
          (bind _returnvalue (Game|SpawnActorfromClass "/Game/Blueprints/GameBlueprint/Sphere_Blueprint.Sphere_Blueprint_C" (Math|Conversions|ToTransform(Vector) (Math|Vector|MakeVector (Utilities|Array|Get(acopy) _all_targets (+ (* _index 5) 2)) (Utilities|Array|Get(acopy) _all_targets (+ (* _index 5) 3)) (Utilities|Array|Get(acopy) _all_targets (+ (* _index 5) 4)))) true 0 0))
          (Variables|/Game/Blueprints/GameBlueprint/Sphere_Blueprint.Sphere_Blueprint_C|Settime_left _returnvalue (* (Utilities|Array|Get(acopy) _all_targets (* _index 5)) (/ 15.0 (Math|Conversions|ToFloat(Integer) (Variables|Default|GetBPM)))))
          (Utilities|Array|RemoveIndex (Variables|Default|Getall_targets) (* _index 5))
          (Utilities|Array|RemoveIndex (Variables|Default|Getall_targets) (* _index 5))
          (Utilities|Array|RemoveIndex (Variables|Default|Getall_targets) (* _index 5))
          (Utilities|Array|RemoveIndex (Variables|Default|Getall_targets) (* _index 5))
          (Utilities|Array|RemoveIndex (Variables|Default|Getall_targets) (* _index 5))))
      ;[1 1 1] Destroy sphere when its time life is ended
      (bind _outactors (Actor|GetAllActorsOfClass "/Game/Blueprints/GameBlueprint/Sphere_Blueprint.Sphere_Blueprint_C"))
      (for _array_element _outactors
        (if (< (Variables|/Game/Blueprints/GameBlueprint/Sphere_Blueprint.Sphere_Blueprint_C|Gettime_left _array_element) 0.0)
          (Default|OnActorDestroy _array_element)
          (Actor|DestroyActor _array_element))))
    (:then_1
      ;[1 1 1] Activate the menu at the end of the level
      (if (> (Utilities|Time|GetGameTimeinSeconds) (Math|Conversions|ToFloat(Integer) (Variables|Default|GetLenght)))
        (Rendering|SetVisibility _staticmeshcomponent true true)
        (for _array_element_2 (Components|GetChildrenComponents _staticmeshcomponent false)
          (bind _asprimitive_component (Utilities|Casting|CastToPrimitiveComponent _array_element_2))
          (Variables|/Script/Engine.PrimitiveComponent|SetbGenerateOverlapEvents _asprimitive_component true))))))

(fn ConstructionScript)