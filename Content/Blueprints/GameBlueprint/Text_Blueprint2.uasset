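; Floating score text actor, a stationary yellow variant of Text_Blueprint that shows briefly and then disappears.
; On Tick, if its text is still empty, it sets a fixed rotation, fills in ScoreText2 and applies the glowing yellow material when Points is zero.
; Tick also counts TimeLeft down to destroy the actor, and rewrites the location with a zero Z offset, leaving it in place.
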(event `self.ReceiveTick`
  (params (DeltaSeconds :type "Float (single-precision)"))
  ;[1 1 1] same as text_blueprint but for the yellow text : go out (not moving and glowing)
  (`|ExecutionSequence`
    (:`then_0`
      (if (`KismetTextLibrary.TextIsEmpty` (`TextRenderComponent.Text` (`self.TextRender`)))
        (`self.SetActorRotation` (struct :`Yaw` 90.0))
        (`TextRenderComponent.K2_SetText` (`self.TextRender`) (`KismetTextLibrary.Conv_StringToText` (`self.score_text2`)))
        (if (== (`self.points`) 0)
          (`PrimitiveComponent.SetMaterial` (`self.TextRender`) 0 "/Game/material/GlowingYellowText.GlowingYellowText"))))
    (:`then_1`
      (bind _output_get (set `self.time_left` (- (`self.time_left`) DeltaSeconds)))
      (if (< _output_get 0.0)
        (`self.K2_DestroyActor`)))
    (:`then_2`
      (`self.K2_SetActorLocation` (`KismetMathLibrary.MakeVector` (.x (`self.K2_GetActorLocation`)) (.y (`self.K2_GetActorLocation`)) (+ (.z (`self.K2_GetActorLocation`)) 0.0))))))

(fn `UserConstructionScript`)